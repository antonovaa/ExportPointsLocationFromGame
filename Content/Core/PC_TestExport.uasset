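; PC_TestExport is a test player controller for login, registration and map travel.
; Pressing R asks GM_TestExport, through a DoOnce gate, to travel to the next map.
; The auth event calls Authorization, then polls GetId on a short delay until a result arrives, printing errors or the user's id and info and blocking further logins after success.
; Registration only forwards its fields and prints a greeting; the test widget setup is unconnected.
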(event `Key|R`
  (params (Key :type "Key Structure"))
  (:`Pressed`
    (`self.travelTo`)))

(event `travelTo`
  (`/Engine/EditorBlueprintResources/StandardMacros.DoOnce` false
    (:`Completed`
      (bind _asgm_test_export (cast `/Game/Core/GM_TestExport` (`GameplayStatics.GetGameMode`)))
      (`/Game/Core/GM_TestExport.TravelToNextMap` _asgm_test_export))))

(event `sendDoAuth`
  (params (login :type String) (password :type String))
  (if (not (`self.isResponse`))
    (`self.Authorization` login password)
    (bind _returnvalue (`self.getId` :!label _label))
    (if (!= _returnvalue -10)
      (bind _returnvalue_2 (`self.getInfo`))
      (`KismetSystemLibrary.Delay` 0.2)
      (if (== _returnvalue -9)
        (`KismetSystemLibrary.PrintString` "backend error" true true (struct :`R` 1.0 :`B` 0.051461 :`A` 1.0) 123.0)
        (elif (== _returnvalue -1)
          (`KismetSystemLibrary.PrintString` "this login not found" true true (struct :`R` 1.0 :`G` 0.0348 :`A` 1.0) 123.0)
          (else
            (set `self.isResponse` true)
            (`KismetSystemLibrary.PrintString` (`KismetStringLibrary.Concat_StrStr` "id=" (`KismetStringLibrary.Conv_IntToString` _returnvalue) " info=" _returnvalue_2) true true (struct :`R` 1.0 :`B` 0.051461 :`A` 1.0) 123.0))))
      (else
        (`KismetSystemLibrary.Delay` 0.2)
        (goto _label)))))

(event `sendDoReg`
  (params (login :type String) (password :type String) (email :type String))
  (`self.Registration` login password email)
  (`KismetSystemLibrary.PrintString` "Hello"))

(event `self.ReceiveBeginPlay`)

(fn `NewFunction_0`)

(fn `UserConstructionScript`)